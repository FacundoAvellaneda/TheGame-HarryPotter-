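; BP_Flipendo is the Flipendo spell actor, which triggers reactions in boxes and turtles it hits.
; On collision overlap it stores its forward vector as ImpactDirection, then branches on the other actor's Box or Tortuga tag.
; It casts to BP_Box or BP_Tortuga and passes itself to that target's interact call.
; It destroys itself after a turtle interaction or untagged overlap, but not after a successful box interaction.
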(event `self.Collision.OnComponentBeginOverlap`
  (params (OverlappedComponent :type "PrimitiveComponent Object Reference") (OtherActor :type "Actor Object Reference") (OtherComp :type "PrimitiveComponent Object Reference") (OtherBodyIndex :type Integer) (bFromSweep :type Boolean) (SweepResult :type "HitResult Structure (by ref)"))
  (set `self.ImpactDirection` (`self.GetActorForwardVector`))
  ;[1 1 1] Interactuar con objetos caja/destruibles
  (if (`self.ActorHasTag` OtherActor "Box")
    (bind _asbp_box (cast `/Game/Blueprints/BP_Box` OtherActor)
      (:`then`
        (`KismetSystemLibrary.PrintString` "Mover")
        (message `/Game/ThirdPerson/Blueprints/BPI_Interactuable.Interact` _asbp_box self))
      (:`CastFailed`
        (`self.K2_DestroyActor` :!label _label)))
    (elif (`self.ActorHasTag` OtherActor "Tortuga")
      (bind _asbp_tortuga (cast `/Game/Blueprints/BP_Tortuga` OtherActor))
      (`/Game/ThirdPerson/Blueprints/BPI_Interactuable.Interact` _asbp_tortuga self)
      (goto _label)
      (else
        (goto _label)))))

(fn `UserConstructionScript`)