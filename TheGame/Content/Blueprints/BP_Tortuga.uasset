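; BP_Tortuga is an interactable physics actor that gets launched when another actor interacts with it.
; Interact applies an impulse to Cube at the actor's location, combining upward JumpForce with AddForce along the caller's velocity direction, then destroys the caller.
; Backup extends the parent version by restoring the original material color, enabling physics simulation and marking the actor movable.
; Debug prints report the cast and resulting impulse.
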(event `/Game/ThirdPerson/Blueprints/BPI_Interactuable.Interact`
  (params (Caller :type "/Game/Blueprints/BP_Flipendo Object Reference"))
  (bind _returnvalue (+ (* (`KismetMathLibrary.Vector_Up`) (`self.JumpForce`)) (* (`KismetMathLibrary.Normal` (`self.GetVelocity` Caller)) (`self.AddForce`))))
  (`KismetSystemLibrary.PrintString` "casteando")
  (`PrimitiveComponent.AddImpulseAtLocation` (`self.Cube`) _returnvalue (`self.K2_GetActorLocation`) "None")
  (`KismetSystemLibrary.PrintString` (`KismetStringLibrary.Conv_VectorToString` _returnvalue))
  (`self.K2_DestroyActor` Caller))

(fn `Backup`
  (bind _cube (`self.Cube`))
  (`parent.Backup`)
  (`MeshComponent.SetVectorParameterValueOnMaterials` _cube "BaseColor" (`KismetMathLibrary.Conv_LinearColorToVector` (`self.OriginalColor`)))
  (`PrimitiveComponent.SetSimulatePhysics` _cube true)
  (set `self.IsMovible` true))

(fn `UserConstructionScript`
  (`parent.UserConstructionScript`))