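; Moving trap actor that, when its Collision component is hit, travels to a target location and returns to where it began play.
; Tick waits a start delay, then eases the actor toward the current target with swept VInterpTo moves.
; Arriving within a small tolerance resets the delay and reverses toward the start, or ends the cycle if already returning.
; Hits during a cycle only print a debug string.
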(event `self.ReceiveBeginPlay`
  (set `self.StartLoccation` (`self.K2_GetActorLocation`)))

(event `self.Collision.OnComponentHit`
  (params (HitComponent :type "PrimitiveComponent Object Reference") (OtherActor :type "Actor Object Reference") (OtherComp :type "PrimitiveComponent Object Reference") (NormalImpulse :type "Vector Structure") (Hit :type "HitResult Structure (by ref)"))
  (if (== (`self.IsMoving`) false)
    (set `self.IsMoving` true)
    (set `self.DelayCounter` 0.0)
    (set `self.IsReturning` false)
    (bind _output_get (set `self.CurrentTarget` (`self.TargetLocation`)))
    (else
      (`KismetSystemLibrary.PrintString` "Nada"))))

(event `self.ReceiveTick`
  (params (DeltaSeconds :type "Float (single-precision)"))
  (bind _returnvalue (`self.K2_GetActorLocation` self))
  (if (== (`self.IsMoving`) true)
    (bind _output_get (set `self.DelayCounter` (+ (`self.DelayCounter`) DeltaSeconds)))
    (if (>= _output_get (`self.TimeToStart`))
      (`self.K2_SetActorLocation` self (`KismetMathLibrary.VInterpTo` _returnvalue (stale `self.Collision.OnComponentHit` _output_get) DeltaSeconds (`self.MoveSpeed`)) true false)
      (if (< (`KismetMathLibrary.VSize` (- (`self.CurrentTarget`) _returnvalue)) 5.0)
        (set `self.DelayCounter` 0.0)
        (if (== (`self.IsReturning`) false)
          (set `self.IsReturning` true)
          (set `self.CurrentTarget` (`self.StartLoccation`))
          (else
            (set `self.IsMoving` false)))))))

(fn `UserConstructionScript`
  (`parent.UserConstructionScript`))