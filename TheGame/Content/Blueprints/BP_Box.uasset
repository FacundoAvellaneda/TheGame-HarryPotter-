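; BP_Box is an interactable physics object that gets pushed when another actor, the Caller, interacts with it.
; Its Interact event applies an impulse to the Door component at the box's location, along the Caller's normalized forward vector scaled by AddForce, then destroys the Caller.
; A separate Backup graph instead takes an overlapping BP_Flipendo's ImpactDirection as the impulse and destroys that actor.
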(event `/Game/ThirdPerson/Blueprints/BPI_Interactuable.Interact`
  (params (Caller :type "/Game/Blueprints/BP_Flipendo Object Reference"))
  (bind _returnvalue (* (`KismetMathLibrary.Normal` (`self.GetActorForwardVector` Caller)) (`self.AddForce`)))
  (`KismetSystemLibrary.PrintString` "casteando")
  (`PrimitiveComponent.AddImpulseAtLocation` (`self.Door`) _returnvalue (`self.K2_GetActorLocation`) "None")
  (`KismetSystemLibrary.PrintString` (`KismetStringLibrary.Conv_VectorToString` _returnvalue))
  (`self.K2_DestroyActor` Caller))

(fn `Backup`
  (bind _overlappingactor (`self.OverlappingActor`))
  (`parent.Backup`)
  (bind _asbp_flipendo (cast `/Game/Blueprints/BP_Flipendo` _overlappingactor))
  (`PrimitiveComponent.AddImpulseAtLocation` (`self.Door`) (`/Game/Blueprints/BP_Flipendo.ImpactDirection` _asbp_flipendo) (`self.K2_GetActorLocation` _overlappingactor) "None")
  (`self.K2_DestroyActor` _overlappingactor))

(fn `UserConstructionScript`
  (`parent.UserConstructionScript`))