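; BP_Door is an interactable door that opens once, becoming passable or see-through through material and collision changes rather than movement.
; On its first Interact event it tints the Door component's materials green, lowers their opacity, switches the collision profile to the NewPerfil variable and prints a debug message.
; An IsOpen flag blocks repeat triggers, and no logic closes the door again.
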(event `/Game/ThirdPerson/Blueprints/BPI_Interactuable.Interact`
  (params (ImpactPoint :type "Vector Structure") (ImpactDirection :type "Vector Structure"))
  (if (not (`self.IsOpen`))
    (`MeshComponent.SetVectorParameterValueOnMaterials` (`self.Door`) "BaseColor" (`KismetMathLibrary.Conv_LinearColorToVector` (make `LinearColor` 0.0 1.0 0.0 1.0)))
    (`MeshComponent.SetScalarParameterValueOnMaterials` (`self.Door`) "Opacity" 0.3)
    (`PrimitiveComponent.SetCollisionProfileName` (`self.Door`) (`self.NewPerfil`) true)
    (`KismetSystemLibrary.PrintString` "Door is open")
    (set `self.IsOpen` true)))

(fn `Backup`)

(fn `UserConstructionScript`
  (`parent.UserConstructionScript`))