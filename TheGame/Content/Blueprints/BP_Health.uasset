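; BP_Health tracks health for a game entity and signals when it dies.
; CurrentHealth starts at MaxHealth on BeginPlay, and TakeDamage subtracts the incoming amount from it.
; At zero or below it calls the OnDeath dispatcher; otherwise it prints the remaining health on screen in green as debug output.
; Health is not clamped, so further hits after death fire OnDeath again.
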(event `self.ReceiveBeginPlay`
  (set `self.CurrentHealth` (`self.MaxHealth`)))

(fn `TakeDamage`
  (params (DamageAmount :type "Float (double-precision)"))
  ;[1 1 1] Funcion para tomar daño
  (bind _output_get (set `self.CurrentHealth` (- (`self.CurrentHealth`) DamageAmount)))
  (if (<= _output_get 0.0)
    (`self.OnDeath`)
    (else
      (`KismetSystemLibrary.PrintString` (`KismetStringLibrary.Conv_DoubleToString` _output_get) true true (struct :`G` 0.354167 :`B` 0.00215 :`A` 1.0)))))